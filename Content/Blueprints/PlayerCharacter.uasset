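; Player character for a top-down stealth action game, with melee attacks, a visible noise ring and a light sensor getter.
; Damage goes to TopDownController, and low health triggers ragdoll, disabled input and game end.
; A timeline animates a dynamic material to show noise radius by loudness, also triggered by G.
; Socket-attached hand spheres drive overlap-and-trace punches with audible hit or miss sounds, while backstabs heavily damage every listed target.
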(event `self.ReceiveAnyDamage`
  (params (Damage :type "Float (single-precision)") (DamageType :type "DamageType Object Reference") (InstigatedBy :type "Controller Object Reference") (DamageCauser :type "Actor Object Reference"))
  (bind _astop_down_controller (cast `/Game/Blueprints/TopDownController` (`self.GetController`)))
  (`/Game/Blueprints/TopDownController.OnCharacterDamage` _astop_down_controller Damage)
  (if (< (`/Game/Blueprints/TopDownController.Health` _astop_down_controller) 1.0)
    (`PrimitiveComponent.SetSimulatePhysics` (`self.Mesh`) true)
    (`self.DisableInput` _astop_down_controller)
    (`CharacterMovementComponent.DisableMovement` _astop_down_controller)
    (bind _astop_down_controller_2 (cast `/Game/Blueprints/TopDownController` (`GameplayStatics.GetPlayerController` null)))
    (set `/Game/Blueprints/TopDownController.Alive` false _astop_down_controller_2)
    (`self.EndGameDispatcher`)))

(event `ShowNoiseCircle`
  (params (Loudness :type "Float (double-precision)" :default 0.0))
  (bind _noiseemittermaterial (`self.NoiseEmitterMaterial`))
  (bind _returnvalue (`KismetMathLibrary.SelectFloat` 0.5 Loudness (`self.BraBool`)))
  ;[1 1 1] NoiseMaking
  (`TimelineComponent.SetPlayRate` (`self.NoiseTest`) (/ 1.0 _returnvalue) :!label _label)
  (`MaterialInstanceDynamic.SetScalarParameterValue` _noiseemittermaterial "MaxDistance" (* _returnvalue 1000.0))
  (bind (_direction _newtrack_1) (`Timeline|NoiseTest` :!via `PlayFromStart`)
    (:`Update`
      (`MaterialInstanceDynamic.SetScalarParameterValue` _noiseemittermaterial "Distance" _newtrack_1))))

(event `Key|G`
  ;[1 1 1] NoiseMaking
  (:`Pressed`
    (set `self.BraBool` false)
    (goto _label))
  (:`Released`
    (set `self.BraBool` true)))

(fn `Backstab Handler`
  (for _array_element (`self.Backstabee`)
    (bind _outhit (`KismetSystemLibrary.LineTraceSingleForObjects` null (`self.K2_GetActorLocation`) (`self.K2_GetActorLocation` _array_element) (`|MakeArray` "ObjectTypeQuery4" :!type "EngineTypes.EObjectTypeQuery Enum")))
    (`GameplayStatics.ApplyPointDamage` _array_element 100.0 (`KismetMathLibrary.MakeVector` 0.0 0.0 -1.0) _outhit null self)))

(fn `GetLightSensitiveComponent`
  (returns (ReturnValue :type "PrimitiveComponent Object Reference"))
  (return (`self.LightSensor`)))

(fn `Punch Handler`
  (params (SphereIn :type "SphereComponent Object Reference") (BoneName :type Name :default "None"))
  (bind _returnvalue (`SceneComponent.K2_GetComponentLocation` SphereIn))
  (bind (_outactors _returnvalue_2) (`KismetSystemLibrary.ComponentOverlapActors_NEW` SphereIn (`SceneComponent.GetSocketTransform` SphereIn BoneName "RTS_World") (`|MakeArray` "ObjectTypeQuery3" :!type "EngineTypes.EObjectTypeQuery Enum") null (`|MakeArray` self :!type "Actor Object Reference")))
  (if _returnvalue_2
    (for _array_element _outactors
      (bind (_outhit _returnvalue_3) (`KismetSystemLibrary.SphereTraceSingleForObjects` null (* _returnvalue 0.7) (* _returnvalue 1.2) (`SphereComponent.SphereRadius` SphereIn) (`|MakeArray` "ObjectTypeQuery4" :!type "EngineTypes.EObjectTypeQuery Enum")))
      (if _returnvalue_3
        (`GameplayStatics.ApplyPointDamage` _array_element 20.0 (`SceneComponent.GetForwardVector` SphereIn) _outhit null self "/Script/Engine.DamageType")
        (`/Game/Blueprints/StaticFunctions.PlaySound` self "/Game/Audio/fx/heavy_punch.heavy_punch" (0.0 0.0 0.0) 1.0 1.0 0.0 null true)))
    (else
      (`/Game/Blueprints/StaticFunctions.PlaySound` self "/Game/Audio/fx/woosh.woosh" _returnvalue 1.0 1.0 0.0 null true))))

(fn `UserConstructionScript`
  (bind _mesh (`self.Mesh`))
  (`|ExecutionSequence`
    (:`then_0`
      (`SceneComponent.K2_AttachTo` (`self.Right Hand Collision Sphere`) _mesh "RightHandSocket" "SnapToTarget" true)
      (`SceneComponent.K2_AttachTo` (`self.Left Hand Collision Sphere`) _mesh "LeftHandSocket" "SnapToTarget" true))
    (:`then_1`
      (bind _returnvalue (`PrimitiveComponent.CreateDynamicMaterialInstance` 0 "/Game/Materials/NoiseEmitterMaterial.NoiseEmitterMaterial"))
      (set `self.NoiseEmitterMaterial` _returnvalue))))