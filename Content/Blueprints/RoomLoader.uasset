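; RoomLoader is a Blueprint that builds parts of a room at runtime from four directional door flags.
; Its GenerateRoom event calls SpawnRoom, which checks NorthDoor, EastDoor, SouthDoor and WestDoor in sequence and adds an automatically attached static mesh component for each one that is true.
; BeginPlay, Tick and the construction script do nothing, so the room only forms when GenerateRoom is called.
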(event `self.ReceiveBeginPlay`)

(event `self.GenerateRoom`
  (`self.SpawnRoom`))

(event `self.ReceiveActorBeginOverlap`
  (params (OtherActor :type "Actor Object Reference")))

(event `self.ReceiveTick`
  (params (DeltaSeconds :type "Float (single-precision)")))

(fn `SpawnRoom`
  (`|ExecutionSequence`
    (:`then_0`
      (if (`self.NorthDoor`)
        (`AddComponent|StaticMeshComponent_9`)))
    (:`then_1`
      (if (`self.EastDoor`)
        (`AddComponent|StaticMeshComponent_10`)))
    (:`then_2`
      (if (`self.SouthDoor`)
        (`AddComponent|StaticMeshComponent_15`)))
    (:`then_3`
      (if (`self.WestDoor`)
        (`AddComponent|StaticMeshComponent_16`)))))

(fn `UserConstructionScript`)