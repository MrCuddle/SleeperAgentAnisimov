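; RoomPrototype1 is a prototype room Blueprint that places doorways on its sides according to four directional door flags.
; The SetDoors event calls GenerateDoors, which checks the North, South, East and West flags in sequence and sets a door-wall static mesh for each enabled side.
; The construction script separately applies a concrete tile material, while door generation runs only through the event.
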(event `self.SetDoors`
  (`self.GenerateDoors`))

(fn `GenerateDoors`
  (`|ExecutionSequence`
    (:`then_0`
      (if (`self.NorthDoor`)
        (`StaticMeshComponent.SetStaticMesh` "/Game/StarterContent/Architecture/Wall_Door_400x300.Wall_Door_400x300")))
    (:`then_1`
      (if (`self.SouthDoor`)
        (`StaticMeshComponent.SetStaticMesh` "/Game/StarterContent/Architecture/Wall_Door_400x300.Wall_Door_400x300")))
    (:`then_2`
      (if (`self.EastDoor`)
        (`StaticMeshComponent.SetStaticMesh` "/Game/StarterContent/Architecture/Wall_Door_400x300.Wall_Door_400x300")))
    (:`then_3`
      (if (`self.WestDoor`)
        (`StaticMeshComponent.SetStaticMesh` "/Game/StarterContent/Architecture/Wall_Door_400x300.Wall_Door_400x300"))))
  (return))

(fn `UserConstructionScript`
  (`PrimitiveComponent.SetMaterial` 0 "/Game/StarterContent/Materials/M_Concrete_Tiles.M_Concrete_Tiles"))