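; DoorWall is an actor with a door that the player opens with the Open Door input action.
; It enables input on BeginPlay and, on a press, checks that the player pawn is within a short distance of the Door component.
; The DoorOpener timeline then plays forward, lerping the door's relative rotation, with no logic to close it.
; TriggerVolume overlaps set an Overlapping flag, which the graph never reads.
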(event `self.TriggerVolume.OnComponentEndOverlap`
  (params (OtherActor :type "Actor Object Reference") (OtherComp :type "PrimitiveComponent Object Reference") (OtherBodyIndex :type Integer))
  (set `self.overlapping` false))

(event `self.TriggerVolume.OnComponentBeginOverlap`
  (params (OtherActor :type "Actor Object Reference") (OtherComp :type "PrimitiveComponent Object Reference") (OtherBodyIndex :type Integer) (bFromSweep :type Boolean) (SweepResult :type "EngineTypes.HitResult Structure (by ref)"))
  (set `self.overlapping` true))

(event `InputAction|Open Door` :consume false
  (:`Pressed`
    (if (< (`KismetMathLibrary.VSize` (- (`self.K2_GetActorLocation` (`GameplayStatics.GetPlayerPawn` 0)) (`SceneComponent.K2_GetComponentLocation` (`self.Door`)))) 150.0)
      (bind (_direction _dooropener) (`Timeline|DoorOpener`)
        (:`Update`
          (`SceneComponent.K2_SetRelativeRotation` (`self.Door`) (`KismetMathLibrary.RLerp` (struct :`Yaw` 90.0) (struct :`Yaw` 180.0) _dooropener true) false))))))

(event `self.ReceiveBeginPlay`
  (`self.EnableInput` (`GameplayStatics.GetPlayerController` null)))

(event `self.ReceiveTick`
  (params (DeltaSeconds :type "Float (single-precision)")))

(fn `UserConstructionScript`)