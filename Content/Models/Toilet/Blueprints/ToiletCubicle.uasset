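; Toilet cubicle prop with a door toggle and a randomly spawned marble-material lid.
; The construction script randomly decides whether to add the lid mesh and records the result in LidSpawned.
; The Open Door input flips Open at any distance, but plays the lock sound only when the player is near the door.
; Timelines for rotating the door exist but are disconnected, so the door never moves.
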(event `self.ReceiveBeginPlay`
  ;[1 1 1] Allow this blueprint to receive input events
  (`self.EnableInput` (`GameplayStatics.GetPlayerController` null)))

(event `self.ReceiveActorBeginOverlap`
  (params (OtherActor :type "Actor Object Reference")))

(event `InputAction|Open Door` :consume false
  (bind _returnvalue (`self.K2_GetActorLocation` (`GameplayStatics.GetPlayerPawn` null)))
  (bind _returnvalue_2 (`SceneComponent.K2_GetComponentLocation` (`self.Door`)))
  (:`Pressed`
    (if (`self.Open`)
      (set `self.Open` false)
      (if (< (`KismetMathLibrary.VSize` (- _returnvalue _returnvalue_2)) 150.0)
        (`GameplayStatics.PlaySoundAtLocation` "/Game/Audio/fx/door-lock-1_Cue.door-lock-1_Cue" (`self.K2_GetActorLocation`) :!label _label))
      (else
        (set `self.Open` true)
        (if (< (`KismetMathLibrary.VSize` (- _returnvalue _returnvalue_2)) 150.0)
          (goto _label))))))

(event `self.ReceiveTick`
  (params (DeltaSeconds :type "Float (single-precision)")))

(fn `UserConstructionScript`
  (switch `int` (`KismetMathLibrary.RandomInteger` 2)
    (:`0`
      (bind _returnvalue (`AddComponent|Static Mesh Component_118` :`RelativeTransform` (`KismetMathLibrary.MakeTransform` (0.0 -76.0 0.0))))
      (`StaticMeshComponent.SetStaticMesh` _returnvalue "/Game/Models/Toilet/Meshes/ToiletLid.ToiletLid")
      (`PrimitiveComponent.SetMaterial` _returnvalue 0 "/Game/StarterContent/Materials/M_Rock_Marble_Polished.M_Rock_Marble_Polished")
      (set `self.LidSpawned` true))
    (:`1`
      (set `self.LidSpawned` false))))