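; Toilet cubicle Blueprint that swings doors open and shut when the player presses the Open Door input.
; The actor enables player input on BeginPlay, then each press loops over an array of components and checks each one's distance to the pawn.
; Two timelines lerp the relative rotation of nearby components through 90 degrees, guarded by a shared AnimationStarted flag.
; The shared Open flag flips for every element, even when out of range or mid-animation.
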(event `self.ReceiveBeginPlay`
  ;[1 1 1] Allow this blueprint to receive input events
  (`self.EnableInput` (`GameplayStatics.GetPlayerController` 0)))

(event `self.ReceiveActorBeginOverlap`
  (params (OtherActor :type "Actor Object Reference")))

(event `self.ReceiveTick`
  (params (DeltaSeconds :type "Float (single-precision)")))

(event `InputAction|Open Door` :consume false
  (bind _returnvalue (`self.K2_GetActorLocation` (`GameplayStatics.GetPlayerPawn` 0)))
  (:`Pressed`
    (for _array_element _
      (if (`self.Open`)
        (set `self.Open` false)
        (bind _returnvalue_2 (`SceneComponent.K2_GetComponentLocation` _array_element))
        (if (< (`KismetMathLibrary.VSize` (- _returnvalue _returnvalue_2)) 150.0)
          (if (not (`self.AnimationStarted`))
            (set `self.AnimationStarted` true)
            (bind (_direction _dooropener) (`Timeline|Timeline_1` :!via `PlayFromStart`)
              (:`Update`
                (`SceneComponent.K2_SetRelativeRotation` _array_element (`KismetMathLibrary.RLerp` (struct) (struct :`Yaw` -90.0) _dooropener true) false))
              (:`Finished`
                (set `self.AnimationStarted` false)))))
        (else
          (set `self.Open` true)
          (if (< (`KismetMathLibrary.VSize` (- _returnvalue _returnvalue_2)) 150.0)
            (if (not (`self.AnimationStarted`))
              (set `self.AnimationStarted` true)
              (bind (_direction_2 _dooropener_2) (`Timeline|Timeline_0` :!via `PlayFromStart`)
                (:`Update`
                  (`SceneComponent.K2_SetRelativeRotation` _array_element (`KismetMathLibrary.RLerp` (struct :`Yaw` -90.0) (struct) _dooropener_2 true) false))
                (:`Finished`
                  (set `self.AnimationStarted` false))))))))))

(fn `UserConstructionScript`)