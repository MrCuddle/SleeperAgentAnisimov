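; Filing cabinet prop that shows one randomly chosen drawer pulled open for visual variety.
; The construction script gathers drawer components 1, 2, 3, 5 and 6 into an array, leaving out drawer 4.
; It moves a random entry along relative Y to open it, building the new location from randomly indexed array lookups.
; The event graph holds only empty events, so there is no runtime behavior.
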(event `self.ReceiveBeginPlay`)

(event `self.ReceiveActorBeginOverlap`
  (params (OtherActor :type "Actor Object Reference")))

(event `self.ReceiveTick`
  (params (DeltaSeconds :type "Float (single-precision)")))

(event `self.FileCabinetDrawer4.OnEndCursorOver`
  (params (TouchedComponent :type "PrimitiveComponent Object Reference")))

(fn `UserConstructionScript`
  (bind _newvar_0 (`self.NewVar_0`))
  (bind _item (`KismetArrayLibrary.Array_Get` _newvar_0 (`KismetMathLibrary.RandomInteger` (`KismetArrayLibrary.Array_Length` _newvar_0))))
  (`KismetArrayLibrary.Array_Add` _newvar_0 (`self.FileCabinetDrawer1`))
  (`KismetArrayLibrary.Array_Add` _newvar_0 (`self.FileCabinetDrawer2`))
  (`KismetArrayLibrary.Array_Add` _newvar_0 (`self.FileCabinetDrawer3`))
  (`KismetArrayLibrary.Array_Add` _newvar_0 (`self.FileCabinetDrawer5`))
  (`KismetArrayLibrary.Array_Add` _newvar_0 (`self.FileCabinetDrawer6`))
  (`SceneComponent.K2_SetRelativeLocation` _item (`KismetMathLibrary.MakeVector` (.x (`SceneComponent.RelativeLocation` _item)) (+ (.y (`SceneComponent.RelativeLocation` _item)) 20.0) (.z (`SceneComponent.RelativeLocation` _item))) false))