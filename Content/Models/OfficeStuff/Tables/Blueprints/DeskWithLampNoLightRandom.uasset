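; Office desk prop Blueprint that places an unlit desk lamp at a random spot on the table.
; The Construction Script rolls a random integer to pick one of three preset positions and angles, then adds a static mesh component with the lamp mesh and a steel material.
; No light component is created and the event graph is empty.
; The roll is unseeded, so placement can change whenever construction reruns.
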(event `self.ReceiveBeginPlay`)

(event `self.ReceiveActorBeginOverlap`
  (params (OtherActor :type "Actor Object Reference")))

(event `self.ReceiveTick`
  (params (DeltaSeconds :type "Float (single-precision)")))

(fn `UserConstructionScript`
  (switch `int` (`KismetMathLibrary.RandomInteger` 3)
    (:`0`
      (bind _returnvalue (`AddComponent|Static Mesh Component_144` :`RelativeTransform` (`KismetMathLibrary.MakeTransform` (70.0 -20.0 85.0) (struct :`Yaw` -135.0))))
      (`StaticMeshComponent.SetStaticMesh` _returnvalue "/Game/Models/OfficeStuff/Lighting/Meshes/DeskLamp.DeskLamp")
      (`PrimitiveComponent.SetMaterial` _returnvalue 0 "/Game/StarterContent/Materials/M_Metal_Steel.M_Metal_Steel"))
    (:`1`
      (bind _returnvalue_2 (`AddComponent|StaticMeshComponent_181` :`RelativeTransform` (`KismetMathLibrary.MakeTransform` (-70.0 -20.0 85.0) (struct :`Yaw` 135.0))))
      (`StaticMeshComponent.SetStaticMesh` _returnvalue_2 "/Game/Models/OfficeStuff/Lighting/Meshes/DeskLamp.DeskLamp")
      (`PrimitiveComponent.SetMaterial` _returnvalue_2 0 "/Game/StarterContent/Materials/M_Metal_Steel.M_Metal_Steel"))
    (:`2`
      (bind _returnvalue_3 (`AddComponent|StaticMeshComponent_166` :`RelativeTransform` (`KismetMathLibrary.MakeTransform` (0.0 -30.0 85.0) (struct :`Yaw` 180.0))))
      (`StaticMeshComponent.SetStaticMesh` _returnvalue_3 "/Game/Models/OfficeStuff/Lighting/Meshes/DeskLamp.DeskLamp")
      (`PrimitiveComponent.SetMaterial` _returnvalue_3 0 "/Game/StarterContent/Materials/M_Metal_Steel.M_Metal_Steel"))))