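; Desk prop that randomizes its file cabinets and desktop clutter in the Construction Script, re-rolling without a seed on each run.
; Nested random switches choose a right, left or no cabinet and its drawer positions; the both-cabinet branch is unreachable with RandomInteger(3).
; All paths converge on one of three desktop layouts with lamp, spot light and in/out box.
; A final roll adds a folder; the computer follows except in one folderless layout.
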(event `self.ReceiveBeginPlay`)

(event `self.ReceiveActorBeginOverlap`
  (params (OtherActor :type "Actor Object Reference")))

(event `self.ReceiveTick`
  (params (DeltaSeconds :type "Float (single-precision)")))

(fn `UserConstructionScript`
  (switch `int` (`KismetMathLibrary.RandomInteger` 3)
    (:`0`
      (bind _returnvalue (`AddComponent|StaticMeshComponent_1120` :`RelativeTransform` (`KismetMathLibrary.MakeTransform` (60.0 20.0 -80.0) (struct) (7.0 7.0 7.0))))
      (`StaticMeshComponent.SetStaticMesh` _returnvalue "/Game/Models/OfficeStuff/FilingCabinets/Meshes/VeryShort2FileCabinet.VeryShort2FileCabinet")
      (`PrimitiveComponent.SetMaterial` _returnvalue 0 "/Game/StarterContent/Materials/M_Metal_Steel.M_Metal_Steel")
      (switch `int` (`KismetMathLibrary.RandomInteger` 4)
        (:`0`
          (bind _returnvalue_2 (`AddComponent|StaticMeshComponent_1122` :`RelativeTransform` (`KismetMathLibrary.MakeTransform` (60.0 55.0 5.0) (struct :`Yaw` 90.0) (7.0 7.8 7.8)) :!label _label))
          (`StaticMeshComponent.SetStaticMesh` _returnvalue_2 "/Game/Models/OfficeStuff/FilingCabinets/Meshes/FileCabinetDrawer1.FileCabinetDrawer1")
          (`PrimitiveComponent.SetMaterial` _returnvalue_2 0 "/Game/StarterContent/Materials/M_Metal_Steel.M_Metal_Steel")
          (bind _returnvalue_3 (`AddComponent|StaticMeshComponent_1124` :`RelativeTransform` (`KismetMathLibrary.MakeTransform` (60.0 55.0 35.0) (struct :`Yaw` 90.0) (7.0 7.8 7.8))))
          (`StaticMeshComponent.SetStaticMesh` _returnvalue_3 "/Game/Models/OfficeStuff/FilingCabinets/Meshes/FileCabinetDrawer1.FileCabinetDrawer1")
          (`PrimitiveComponent.SetMaterial` _returnvalue_3 0 "/Game/StarterContent/Materials/M_Metal_Steel.M_Metal_Steel"))
        (:`1`
          (bind _returnvalue_4 (`AddComponent|StaticMeshComponent_1126` :`RelativeTransform` (`KismetMathLibrary.MakeTransform` (60.0 55.0 5.0) (struct :`Yaw` 90.0) (7.0 7.8 7.8))))
          (`StaticMeshComponent.SetStaticMesh` _returnvalue_4 "/Game/Models/OfficeStuff/FilingCabinets/Meshes/FileCabinetDrawer1.FileCabinetDrawer1")
          (`PrimitiveComponent.SetMaterial` _returnvalue_4 0 "/Game/StarterContent/Materials/M_Metal_Steel.M_Metal_Steel")
          (bind _returnvalue_5 (`AddComponent|StaticMeshComponent_1127` :`RelativeTransform` (`KismetMathLibrary.MakeTransform` (60.0 75.0 35.0) (struct :`Yaw` 90.0) (7.0 7.8 7.8))))
          (`StaticMeshComponent.SetStaticMesh` _returnvalue_5 "/Game/Models/OfficeStuff/FilingCabinets/Meshes/FileCabinetDrawer1.FileCabinetDrawer1")
          (`PrimitiveComponent.SetMaterial` _returnvalue_5 0 "/Game/StarterContent/Materials/M_Metal_Steel.M_Metal_Steel"))
        (:`2`
          (bind _returnvalue_6 (`AddComponent|StaticMeshComponent_1128` :`RelativeTransform` (`KismetMathLibrary.MakeTransform` (60.0 75.0 5.0) (struct :`Yaw` 90.0) (7.0 7.8 7.8))))
          (`StaticMeshComponent.SetStaticMesh` _returnvalue_6 "/Game/Models/OfficeStuff/FilingCabinets/Meshes/FileCabinetDrawer1.FileCabinetDrawer1")
          (`PrimitiveComponent.SetMaterial` _returnvalue_6 0 "/Game/StarterContent/Materials/M_Metal_Steel.M_Metal_Steel")
          (bind _returnvalue_7 (`AddComponent|StaticMeshComponent_1129` :`RelativeTransform` (`KismetMathLibrary.MakeTransform` (60.0 55.0 35.0) (struct :`Yaw` 90.0) (7.0 7.8 7.8))))
          (`StaticMeshComponent.SetStaticMesh` _returnvalue_7 "/Game/Models/OfficeStuff/FilingCabinets/Meshes/FileCabinetDrawer1.FileCabinetDrawer1")
          (`PrimitiveComponent.SetMaterial` _returnvalue_7 0 "/Game/StarterContent/Materials/M_Metal_Steel.M_Metal_Steel"))
        (:`3`
          (goto _label))))
    (:`1`
      (bind _returnvalue_8 (`AddComponent|StaticMeshComponent_1121` :`RelativeTransform` (`KismetMathLibrary.MakeTransform` (-60.0 20.0 -80.0) (struct) (7.0 7.0 7.0))))
      (`StaticMeshComponent.SetStaticMesh` _returnvalue_8 "/Game/Models/OfficeStuff/FilingCabinets/Meshes/VeryShort2FileCabinet.VeryShort2FileCabinet")
      (`PrimitiveComponent.SetMaterial` _returnvalue_8 0 "/Game/StarterContent/Materials/M_Metal_Steel.M_Metal_Steel")
      (switch `int` (`KismetMathLibrary.RandomInteger` 4)
        (:`0`
          (bind _returnvalue_9 (`AddComponent|StaticMeshComponent_1123` :`RelativeTransform` (`KismetMathLibrary.MakeTransform` (-60.0 55.0 5.0) (struct :`Yaw` 90.0) (7.8 7.8 7.8)) :!label _label_2))
          (`StaticMeshComponent.SetStaticMesh` _returnvalue_9 "/Game/Models/OfficeStuff/FilingCabinets/Meshes/FileCabinetDrawer1.FileCabinetDrawer1")
          (`PrimitiveComponent.SetMaterial` _returnvalue_9 0 "/Game/StarterContent/Materials/M_Metal_Steel.M_Metal_Steel")
          (bind _returnvalue_10 (`AddComponent|StaticMeshComponent_1125` :`RelativeTransform` (`KismetMathLibrary.MakeTransform` (-60.0 55.0 35.0) (struct :`Yaw` 90.0) (7.8 7.8 7.8))))
          (`StaticMeshComponent.SetStaticMesh` _returnvalue_10 "/Game/Models/OfficeStuff/FilingCabinets/Meshes/FileCabinetDrawer1.FileCabinetDrawer1")
          (`PrimitiveComponent.SetMaterial` _returnvalue_10 0 "/Game/StarterContent/Materials/M_Metal_Steel.M_Metal_Steel"))
        (:`1`
          (bind _returnvalue_11 (`AddComponent|StaticMeshComponent_1130` :`RelativeTransform` (`KismetMathLibrary.MakeTransform` (-60.0 55.0 5.0) (struct :`Yaw` 90.0) (7.8 7.8 7.8))))
          (`StaticMeshComponent.SetStaticMesh` _returnvalue_11 "/Game/Models/OfficeStuff/FilingCabinets/Meshes/FileCabinetDrawer1.FileCabinetDrawer1")
          (`PrimitiveComponent.SetMaterial` _returnvalue_11 0 "/Game/StarterContent/Materials/M_Metal_Steel.M_Metal_Steel")
          (bind _returnvalue_12 (`AddComponent|StaticMeshComponent_1131` :`RelativeTransform` (`KismetMathLibrary.MakeTransform` (-60.0 75.0 35.0) (struct :`Yaw` 90.0) (7.8 7.8 7.8))))
          (`StaticMeshComponent.SetStaticMesh` _returnvalue_12 "/Game/Models/OfficeStuff/FilingCabinets/Meshes/FileCabinetDrawer1.FileCabinetDrawer1")
          (`PrimitiveComponent.SetMaterial` _returnvalue_12 0 "/Game/StarterContent/Materials/M_Metal_Steel.M_Metal_Steel"))
        (:`2`
          (bind _returnvalue_13 (`AddComponent|StaticMeshComponent_1132` :`RelativeTransform` (`KismetMathLibrary.MakeTransform` (-60.0 75.0 5.0) (struct :`Yaw` 90.0) (7.8 7.8 7.8))))
          (`StaticMeshComponent.SetStaticMesh` _returnvalue_13 "/Game/Models/OfficeStuff/FilingCabinets/Meshes/FileCabinetDrawer1.FileCabinetDrawer1")
          (`PrimitiveComponent.SetMaterial` _returnvalue_13 0 "/Game/StarterContent/Materials/M_Metal_Steel.M_Metal_Steel")
          (bind _returnvalue_14 (`AddComponent|StaticMeshComponent_1133` :`RelativeTransform` (`KismetMathLibrary.MakeTransform` (-60.0 55.0 35.0) (struct :`Yaw` 90.0) (7.8 7.8 7.8))))
          (`StaticMeshComponent.SetStaticMesh` _returnvalue_14 "/Game/Models/OfficeStuff/FilingCabinets/Meshes/FileCabinetDrawer1.FileCabinetDrawer1")
          (`PrimitiveComponent.SetMaterial` _returnvalue_14 0 "/Game/StarterContent/Materials/M_Metal_Steel.M_Metal_Steel"))
        (:`3`
          (goto _label_2))))
    (:`2`
      _)
    (:`3`
      (bind _returnvalue_15 (`AddComponent|StaticMeshComponent_1134` :`RelativeTransform` (`KismetMathLibrary.MakeTransform` (-60.0 20.0 -80.0) (struct) (7.0 7.0 7.0))))
      (`StaticMeshComponent.SetStaticMesh` _returnvalue_15 "/Game/Models/OfficeStuff/FilingCabinets/Meshes/VeryShort2FileCabinet.VeryShort2FileCabinet")
      (`PrimitiveComponent.SetMaterial` _returnvalue_15 0 "/Game/StarterContent/Materials/M_Metal_Steel.M_Metal_Steel")
      (switch `int` (`KismetMathLibrary.RandomInteger` 4)
        (:`0`
          (bind _returnvalue_16 (`AddComponent|StaticMeshComponent_1135` :`RelativeTransform` (`KismetMathLibrary.MakeTransform` (-60.0 55.0 5.0) (struct :`Yaw` 90.0) (7.8 7.8 7.8)) :!label _label_3))
          (`StaticMeshComponent.SetStaticMesh` _returnvalue_16 "/Game/Models/OfficeStuff/FilingCabinets/Meshes/FileCabinetDrawer1.FileCabinetDrawer1")
          (`PrimitiveComponent.SetMaterial` _returnvalue_16 0 "/Game/StarterContent/Materials/M_Metal_Steel.M_Metal_Steel")
          (bind _returnvalue_17 (`AddComponent|StaticMeshComponent_1136` :`RelativeTransform` (`KismetMathLibrary.MakeTransform` (-60.0 55.0 35.0) (struct :`Yaw` 90.0) (7.8 7.8 7.8))))
          (`StaticMeshComponent.SetStaticMesh` _returnvalue_17 "/Game/Models/OfficeStuff/FilingCabinets/Meshes/FileCabinetDrawer1.FileCabinetDrawer1")
          (`PrimitiveComponent.SetMaterial` _returnvalue_17 0 "/Game/StarterContent/Materials/M_Metal_Steel.M_Metal_Steel"))
        (:`1`
          (bind _returnvalue_18 (`AddComponent|StaticMeshComponent_1137` :`RelativeTransform` (`KismetMathLibrary.MakeTransform` (-60.0 55.0 5.0) (struct :`Yaw` 90.0) (7.8 7.8 7.8))))
          (`StaticMeshComponent.SetStaticMesh` _returnvalue_18 "/Game/Models/OfficeStuff/FilingCabinets/Meshes/FileCabinetDrawer1.FileCabinetDrawer1")
          (`PrimitiveComponent.SetMaterial` _returnvalue_18 0 "/Game/StarterContent/Materials/M_Metal_Steel.M_Metal_Steel")
          (bind _returnvalue_19 (`AddComponent|StaticMeshComponent_1138` :`RelativeTransform` (`KismetMathLibrary.MakeTransform` (-60.0 75.0 35.0) (struct :`Yaw` 90.0) (7.8 7.8 7.8))))
          (`StaticMeshComponent.SetStaticMesh` _returnvalue_19 "/Game/Models/OfficeStuff/FilingCabinets/Meshes/FileCabinetDrawer1.FileCabinetDrawer1")
          (`PrimitiveComponent.SetMaterial` _returnvalue_19 0 "/Game/StarterContent/Materials/M_Metal_Steel.M_Metal_Steel"))
        (:`2`
          (bind _returnvalue_20 (`AddComponent|StaticMeshComponent_1139` :`RelativeTransform` (`KismetMathLibrary.MakeTransform` (-60.0 75.0 5.0) (struct :`Yaw` 90.0) (7.8 7.8 7.8))))
          (`StaticMeshComponent.SetStaticMesh` _returnvalue_20 "/Game/Models/OfficeStuff/FilingCabinets/Meshes/FileCabinetDrawer1.FileCabinetDrawer1")
          (`PrimitiveComponent.SetMaterial` _returnvalue_20 0 "/Game/StarterContent/Materials/M_Metal_Steel.M_Metal_Steel")
          (bind _returnvalue_21 (`AddComponent|StaticMeshComponent_1140` :`RelativeTransform` (`KismetMathLibrary.MakeTransform` (-60.0 55.0 35.0) (struct :`Yaw` 90.0) (7.8 7.8 7.8))))
          (`StaticMeshComponent.SetStaticMesh` _returnvalue_21 "/Game/Models/OfficeStuff/FilingCabinets/Meshes/FileCabinetDrawer1.FileCabinetDrawer1")
          (`PrimitiveComponent.SetMaterial` _returnvalue_21 0 "/Game/StarterContent/Materials/M_Metal_Steel.M_Metal_Steel"))
        (:`3`
          (goto _label_3)))
      (bind _returnvalue_22 (`AddComponent|StaticMeshComponent_1141` :`RelativeTransform` (`KismetMathLibrary.MakeTransform` (60.0 20.0 -80.0) (struct) (7.0 7.0 7.0))))
      (`StaticMeshComponent.SetStaticMesh` _returnvalue_22 "/Game/Models/OfficeStuff/FilingCabinets/Meshes/VeryShort2FileCabinet.VeryShort2FileCabinet")
      (`PrimitiveComponent.SetMaterial` _returnvalue_22 0 "/Game/StarterContent/Materials/M_Metal_Steel.M_Metal_Steel")
      (switch `int` (`KismetMathLibrary.RandomInteger` 4)
        (:`0`
          (bind _returnvalue_23 (`AddComponent|StaticMeshComponent_1142` :`RelativeTransform` (`KismetMathLibrary.MakeTransform` (60.0 55.0 5.0) (struct :`Yaw` 90.0) (7.0 7.8 7.8)) :!label _label_4))
          (`StaticMeshComponent.SetStaticMesh` _returnvalue_23 "/Game/Models/OfficeStuff/FilingCabinets/Meshes/FileCabinetDrawer1.FileCabinetDrawer1")
          (`PrimitiveComponent.SetMaterial` _returnvalue_23 0 "/Game/StarterContent/Materials/M_Metal_Steel.M_Metal_Steel")
          (bind _returnvalue_24 (`AddComponent|StaticMeshComponent_1143` :`RelativeTransform` (`KismetMathLibrary.MakeTransform` (60.0 55.0 35.0) (struct :`Yaw` 90.0) (7.0 7.8 7.8))))
          (`StaticMeshComponent.SetStaticMesh` _returnvalue_24 "/Game/Models/OfficeStuff/FilingCabinets/Meshes/FileCabinetDrawer1.FileCabinetDrawer1")
          (`PrimitiveComponent.SetMaterial` _returnvalue_24 0 "/Game/StarterContent/Materials/M_Metal_Steel.M_Metal_Steel"))
        (:`1`
          (bind _returnvalue_25 (`AddComponent|StaticMeshComponent_1144` :`RelativeTransform` (`KismetMathLibrary.MakeTransform` (60.0 55.0 5.0) (struct :`Yaw` 90.0) (7.0 7.8 7.8))))
          (`StaticMeshComponent.SetStaticMesh` _returnvalue_25 "/Game/Models/OfficeStuff/FilingCabinets/Meshes/FileCabinetDrawer1.FileCabinetDrawer1")
          (`PrimitiveComponent.SetMaterial` _returnvalue_25 0 "/Game/StarterContent/Materials/M_Metal_Steel.M_Metal_Steel")
          (bind _returnvalue_26 (`AddComponent|StaticMeshComponent_1145` :`RelativeTransform` (`KismetMathLibrary.MakeTransform` (60.0 75.0 35.0) (struct :`Yaw` 90.0) (7.0 7.8 7.8))))
          (`StaticMeshComponent.SetStaticMesh` _returnvalue_26 "/Game/Models/OfficeStuff/FilingCabinets/Meshes/FileCabinetDrawer1.FileCabinetDrawer1")
          (`PrimitiveComponent.SetMaterial` _returnvalue_26 0 "/Game/StarterContent/Materials/M_Metal_Steel.M_Metal_Steel"))
        (:`2`
          (bind _returnvalue_27 (`AddComponent|StaticMeshComponent_1146` :`RelativeTransform` (`KismetMathLibrary.MakeTransform` (60.0 75.0 5.0) (struct :`Yaw` 90.0) (7.0 7.8 7.8))))
          (`StaticMeshComponent.SetStaticMesh` _returnvalue_27 "/Game/Models/OfficeStuff/FilingCabinets/Meshes/FileCabinetDrawer1.FileCabinetDrawer1")
          (`PrimitiveComponent.SetMaterial` _returnvalue_27 0 "/Game/StarterContent/Materials/M_Metal_Steel.M_Metal_Steel")
          (bind _returnvalue_28 (`AddComponent|StaticMeshComponent_1147` :`RelativeTransform` (`KismetMathLibrary.MakeTransform` (60.0 55.0 35.0) (struct :`Yaw` 90.0) (7.0 7.8 7.8))))
          (`StaticMeshComponent.SetStaticMesh` _returnvalue_28 "/Game/Models/OfficeStuff/FilingCabinets/Meshes/FileCabinetDrawer1.FileCabinetDrawer1")
          (`PrimitiveComponent.SetMaterial` _returnvalue_28 0 "/Game/StarterContent/Materials/M_Metal_Steel.M_Metal_Steel"))
        (:`3`
          (goto _label_4)))))
  (switch `int` (`KismetMathLibrary.RandomInteger` 3)
    (:`0`
      ;[1 1 1] ItemOnDesk Randomizer
      (bind _returnvalue_29 (`AddComponent|StaticMeshComponent_1111` :`RelativeTransform` (`KismetMathLibrary.MakeTransform` (70.0 -20.0 85.0) (struct :`Yaw` -135.0))))
      (`StaticMeshComponent.SetStaticMesh` _returnvalue_29 "/Game/Models/OfficeStuff/Lighting/Meshes/DeskLamp.DeskLamp")
      (`PrimitiveComponent.SetMaterial` _returnvalue_29 0 "/Game/StarterContent/Materials/M_Metal_Steel.M_Metal_Steel")
      (`AddComponent|SpotLightComponent_0` :`RelativeTransform` (`KismetMathLibrary.MakeTransform` (53.0 -5.0 128.0) (struct :`Pitch` -65.0 :`Yaw` 135.0 :`Roll` -92.0)))
      (bind _returnvalue_30 (`AddComponent|StaticMeshComponent_1114` :`RelativeTransform` (`KismetMathLibrary.MakeTransform` (-70.0 -20.0 85.0) (struct :`Yaw` -20.0) (1.3 1.3 1.3))))
      (`StaticMeshComponent.SetStaticMesh` _returnvalue_30 "/Game/Models/OfficeStuff/Misc/Meshes/InOutBox.InOutBox")
      (`PrimitiveComponent.SetMaterial` _returnvalue_30 0 "/Game/StarterContent/Materials/M_Metal_Steel.M_Metal_Steel")
      (switch `int` (`KismetMathLibrary.RandomInteger` 2)
        (:`0`
          (bind _returnvalue_31 (`AddComponent|StaticMeshComponent_1117` :`RelativeTransform` (`KismetMathLibrary.MakeTransform` (-60.0 -15.0 90.0) (struct :`Yaw` -20.0) (1.0 1.0 1.0))))
          (`StaticMeshComponent.SetStaticMesh` _returnvalue_31 "/Game/Models/OfficeStuff/Misc/Meshes/Folder.Folder")
          (`PrimitiveComponent.SetMaterial` _returnvalue_31 0 "/Game/StarterContent/Materials/M_Metal_Gold.M_Metal_Gold")
          ;[1 1 1] ComputerOnDesk
          (bind _returnvalue_32 (`AddComponent|StaticMeshComponent_1149` :`RelativeTransform` (`KismetMathLibrary.MakeTransform` (0.0 -30.0 75.0) (struct :`Yaw` -90.0) (1.0 1.0 1.0)) :!label _label_5))
          (`StaticMeshComponent.SetStaticMesh` _returnvalue_32 "/Game/Models/OfficeStuff/Tech/Meshes/computer.computer")
          (`PrimitiveComponent.SetMaterial` _returnvalue_32 0 "/Game/StarterContent/Materials/M_Wood_Walnut.M_Wood_Walnut"))))
    (:`1`
      (bind _returnvalue_33 (`AddComponent|StaticMeshComponent_1113` :`RelativeTransform` (`KismetMathLibrary.MakeTransform` (-70.0 -20.0 85.0) (struct :`Yaw` 135.0))))
      (`StaticMeshComponent.SetStaticMesh` _returnvalue_33 "/Game/Models/OfficeStuff/Lighting/Meshes/DeskLamp.DeskLamp")
      (`PrimitiveComponent.SetMaterial` _returnvalue_33 0 "/Game/StarterContent/Materials/M_Metal_Steel.M_Metal_Steel")
      (`AddComponent|SpotLightComponent_1` :`RelativeTransform` (`KismetMathLibrary.MakeTransform` (-53.0 -5.0 128.0) (struct :`Pitch` -65.0 :`Yaw` 45.0 :`Roll` -92.0)))
      (bind _returnvalue_34 (`AddComponent|StaticMeshComponent_1116` :`RelativeTransform` (`KismetMathLibrary.MakeTransform` (60.0 -20.0 85.0) (struct :`Yaw` 10.0) (1.3 1.3 1.3))))
      (`StaticMeshComponent.SetStaticMesh` _returnvalue_34 "/Game/Models/OfficeStuff/Misc/Meshes/InOutBox.InOutBox")
      (`PrimitiveComponent.SetMaterial` _returnvalue_34 0 "/Game/StarterContent/Materials/M_Metal_Steel.M_Metal_Steel")
      (switch `int` (`KismetMathLibrary.RandomInteger` 2)
        (:`0`
          (bind _returnvalue_35 (`AddComponent|StaticMeshComponent_1118` :`RelativeTransform` (`KismetMathLibrary.MakeTransform` (65.0 -15.0 90.0) (struct :`Yaw` 10.0) (1.0 1.0 1.0))))
          (`StaticMeshComponent.SetStaticMesh` _returnvalue_35 "/Game/Models/OfficeStuff/Misc/Meshes/Folder.Folder")
          (`PrimitiveComponent.SetMaterial` _returnvalue_35 0 "/Game/StarterContent/Materials/M_Metal_Gold.M_Metal_Gold")
          (goto _label_5))
        (:`1`
          (goto _label_5))))
    (:`2`
      (bind _returnvalue_36 (`AddComponent|StaticMeshComponent_1112` :`RelativeTransform` (`KismetMathLibrary.MakeTransform` (0.0 -30.0 85.0) (struct :`Yaw` 180.0))))
      (`StaticMeshComponent.SetStaticMesh` _returnvalue_36 "/Game/Models/OfficeStuff/Lighting/Meshes/DeskLamp.DeskLamp")
      (`PrimitiveComponent.SetMaterial` _returnvalue_36 0 "/Game/StarterContent/Materials/M_Metal_Steel.M_Metal_Steel")
      ;;[1 1 1] Comment
      (`AddComponent|SpotLightComponent_2` :`RelativeTransform` (`KismetMathLibrary.MakeTransform` (0.0 -10.0 128.0) (struct :`Pitch` -65.0 :`Yaw` 90.0 :`Roll` -92.0)))
      (bind _returnvalue_37 (`AddComponent|StaticMeshComponent_1115` :`RelativeTransform` (`KismetMathLibrary.MakeTransform` (60.0 -20.0 85.0) (struct :`Yaw` 10.0) (1.3 1.3 1.3))))
      (`StaticMeshComponent.SetStaticMesh` _returnvalue_37 "/Game/Models/OfficeStuff/Misc/Meshes/InOutBox.InOutBox")
      (`PrimitiveComponent.SetMaterial` _returnvalue_37 0 "/Game/StarterContent/Materials/M_Metal_Steel.M_Metal_Steel")
      (switch `int` (`KismetMathLibrary.RandomInteger` 2)
        (:`0`
          (bind _returnvalue_38 (`AddComponent|StaticMeshComponent_1119` :`RelativeTransform` (`KismetMathLibrary.MakeTransform` (65.0 -15.0 90.0) (struct :`Yaw` 10.0) (1.0 1.0 1.0))))
          (`StaticMeshComponent.SetStaticMesh` _returnvalue_38 "/Game/Models/OfficeStuff/Misc/Meshes/Folder.Folder")
          (`PrimitiveComponent.SetMaterial` _returnvalue_38 0 "/Game/StarterContent/Materials/M_Metal_Gold.M_Metal_Gold"))
        (:`1`
          _))
      (bind _returnvalue_39 (`AddComponent|StaticMeshComponent_1150` :`RelativeTransform` (`KismetMathLibrary.MakeTransform` (-70.0 -20.0 75.0) (struct :`Yaw` -120.0))))
      (`StaticMeshComponent.SetStaticMesh` _returnvalue_39 "/Game/Models/OfficeStuff/Tech/Meshes/computer.computer")
      (`PrimitiveComponent.SetMaterial` _returnvalue_39 0 "/Game/StarterContent/Materials/M_Wood_Walnut.M_Wood_Walnut"))))